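; BP_FinalBoss is a final boss character that dies when the side-scrolling player character overlaps its capsule.
; The overlap prints a debug message and calls Die, which stops its Manager and zeroes movement velocity.
; Die then switches the mesh to the Ragdoll profile, simulates physics on capsule and mesh, launches both with a fixed impulse and destroys the actor after a short delay.
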(event `self.CapsuleComponent.OnComponentBeginOverlap`
  (params (OverlappedComponent :type "PrimitiveComponent Object Reference") (OtherActor :type "Actor Object Reference") (OtherComp :type "PrimitiveComponent Object Reference") (OtherBodyIndex :type Integer) (bFromSweep :type Boolean) (SweepResult :type "HitResult Structure (by ref)"))
  (cast `/Game/Variant_SideScroller/Blueprints/BP_SideScrollingCharacter` OtherActor)
  (`KismetSystemLibrary.PrintString` "Got 'em" true true (struct :`R` 1.0 :`G` 0.260886 :`B` 0.131445 :`A` 1.0))
  (`self.Die`))

(event `Die`
  (`/Game/ObstacleAttacks/BP_AttackManager.Stop!` (`self.Manager`))
  (`PrimitiveComponent.SetCollisionEnabled` (`self.Mesh`) "QueryAndPhysics")
  (`PrimitiveComponent.SetCollisionEnabled` (`self.CapsuleComponent`) "QueryAndPhysics")
  (set `MovementComponent.Velocity` (0.0 0.0 0.0) (`self.CharacterMovement`))
  (`PrimitiveComponent.SetCollisionProfileName` (`self.Mesh`) "Ragdoll" true)
  (`PrimitiveComponent.SetSimulatePhysics` (`self.CapsuleComponent`) true)
  (`PrimitiveComponent.SetSimulatePhysics` (`self.Mesh`) true)
  (`PrimitiveComponent.AddImpulse` (`self.CapsuleComponent`) (5555.0 6666.0 555.0) "None" true)
  (`PrimitiveComponent.AddImpulse` (`self.Mesh`) (5555.0 6666.0 555.0) "None" true)
  (`KismetSystemLibrary.Delay` 3.0)
  (`self.K2_DestroyActor`))

(fn `UserConstructionScript`)