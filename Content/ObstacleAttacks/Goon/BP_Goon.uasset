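; BP_Goon is an obstacle-attack character that charges toward a target point when its Attack! event fires, with a grunt sound.
; It uses AIMoveTo to reach the target and destroys itself on arrival, on failure, or after a short delay.
; Overlapping the side-scrolling player applies damage and triggers Die, which switches on ragdoll physics, launches capsule and mesh with an impulse, then destroys the goon.
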(event `Attack!`
  (`GameplayStatics.PlaySoundAtLocation` "/Game/Audio/AE_UltraGrunt.AE_UltraGrunt" (`SceneComponent.RelativeLocation` (`self.CapsuleComponent`)) (struct) 1.0 1.0 0.0 null null null null)
  (`|AIMoveTo` self (0.0 0.0 0.0) (`self.Target Point`)
    (:`then`
      (`KismetSystemLibrary.Delay` 4.0)
      (`self.K2_DestroyActor`))
    (:`OnSuccess`
      (`KismetSystemLibrary.PrintString` "Made it")
      (`self.K2_DestroyActor`))
    (:`OnFail`
      (`self.K2_DestroyActor`))))

(event `self.CapsuleComponent.OnComponentBeginOverlap`
  (params (OverlappedComponent :type "PrimitiveComponent Object Reference") (OtherActor :type "Actor Object Reference") (OtherComp :type "PrimitiveComponent Object Reference") (OtherBodyIndex :type Integer) (bFromSweep :type Boolean) (SweepResult :type "HitResult Structure (by ref)"))
  (cast `/Game/Variant_SideScroller/Blueprints/BP_SideScrollingCharacter` OtherActor)
  (`GameplayStatics.ApplyDamage` OtherActor 50.0)
  (`KismetSystemLibrary.PrintString` "Got 'em" true true (struct :`R` 1.0 :`G` 0.260886 :`B` 0.131445 :`A` 1.0))
  (`self.Die`))

(event `Die`
  (`PrimitiveComponent.SetCollisionEnabled` (`self.Mesh`) "QueryAndPhysics")
  (`PrimitiveComponent.SetCollisionEnabled` (`self.CapsuleComponent`) "QueryAndPhysics")
  (set `MovementComponent.Velocity` (0.0 0.0 0.0) (`self.CharacterMovement`))
  (`PrimitiveComponent.SetCollisionProfileName` (`self.Mesh`) "Ragdoll" true)
  (`PrimitiveComponent.SetSimulatePhysics` (`self.CapsuleComponent`) true)
  (`PrimitiveComponent.SetSimulatePhysics` (`self.Mesh`) true)
  (`PrimitiveComponent.AddImpulse` (`self.CapsuleComponent`) (5555.0 6666.0 555.0) "None" true)
  (`PrimitiveComponent.AddImpulse` (`self.Mesh`) (5555.0 6666.0 555.0) "None" true)
  (`KismetSystemLibrary.Delay` 3.0)
  (`self.K2_DestroyActor`))

(fn `UserConstructionScript`)