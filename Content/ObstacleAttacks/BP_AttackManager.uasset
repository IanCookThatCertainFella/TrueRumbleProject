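; Attack manager that runs an endless loop of obstacle attacks against the player, starting at BeginPlay.
; A random looping MultiGate picks Quake, Projectile, Slammer or SpawnGoon, and each picks again after a random delay.
; Projectiles and goons spawn offset from the player, while Quake builds camera shake and rumble, sparing airborne players from DoDamage.
; Damage is placeholder: DoDamage only prints, ApplyDamage calls have no target, and Slammer has no visible attack.
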(event `Projectile`
  (bind _returnvalue (`SceneComponent.GetRelativeTransform` (`Actor.RootComponent` (`GameplayStatics.GetPlayerCharacter` 0))))
  (`KismetSystemLibrary.PrintString` "Bang!")
  (`|SpawnActorFromClass` "/Game/ObstacleAttacks/BP_Projectile.BP_Projectile_C" (`KismetMathLibrary.MakeTransform` (`KismetMathLibrary.MakeVector` (+ (.x (.location _returnvalue)) 800.0) (.y (.location _returnvalue)) 600.0) (struct :`Yaw` 180.0)) "Undefined" "MultiplyWithRoot" null null)
  (bind _output_get (set `self.Attack Delay` (`KismetMathLibrary.RandomFloatInRange` 0.5 2.0)))
  (`KismetSystemLibrary.Delay` _output_get)
  (`GameplayStatics.ApplyDamage` null 10.0)
  (`self.Decide Next Attack`))

(event `Slammer`
  (`KismetSystemLibrary.PrintString` "Urgh!")
  (bind _output_get (set `self.Attack Delay` (`KismetMathLibrary.RandomFloatInRange` 0.5 2.0)))
  (`KismetSystemLibrary.Delay` _output_get)
  (`GameplayStatics.ApplyDamage` null 10.0)
  (`self.Decide Next Attack`))

(event `Do Damage`
  (`KismetSystemLibrary.PrintString` "Yowch!"))

(event `Spawn Goon`
  (bind _returnvalue (`SceneComponent.GetRelativeTransform` (`Actor.RootComponent` (`GameplayStatics.GetPlayerCharacter` 0))))
  (`KismetSystemLibrary.PrintString` "Bad Joke!")
  (`KismetSystemLibrary.Delay` 2.0)
  (bind _returnvalue_2 (`|SpawnActorFromClass` "/Game/ObstacleAttacks/Goon/BP_Goon.BP_Goon_C" (`KismetMathLibrary.MakeTransform` (`KismetMathLibrary.MakeVector` (+ (.x (.location _returnvalue)) 800.0) (.y (.location _returnvalue)) 500.0) (.rotation _returnvalue) (.scale _returnvalue)) "Undefined" "MultiplyWithRoot" null null))
  (set `/Game/ObstacleAttacks/Goon/BP_Goon.Manager` self _returnvalue_2)
  (set `/Game/ObstacleAttacks/Goon/BP_Goon.Target Point` (`self.Target Point`) _returnvalue_2)
  (`/Game/ObstacleAttacks/Goon/BP_Goon.Attack!` _returnvalue_2)
  (bind _output_get (set `self.Attack Delay` (`KismetMathLibrary.RandomFloatInRange` 0.5 2.0)))
  (`KismetSystemLibrary.Delay` _output_get)
  (`self.Decide Next Attack`))

(event `Decide Next Attack`
  (`|MultiGate` true true
    (:`Out 0`
      (`self.Quake`))
    (:`Out 1`
      (`self.Projectile`))
    (:`Out 2`
      (`self.Slammer`))
    (:`Out 3`
      (`self.Spawn Goon`))))

(event `self.ReceiveBeginPlay`
  (`self.Decide Next Attack`))

(event `Quake`
  (bind _returnvalue (`GameplayStatics.GetPlayerCharacter` 0))
  (bind _capsulecomponent (`Character.CapsuleComponent` _returnvalue))
  (`KismetSystemLibrary.PrintString` "Grumble")
  (`LegacyCameraShake.StartLegacyCameraShake` (`GameplayStatics.GetPlayerCameraManager` 0) "/Game/CameraShake/LCS_Quake.LCS_Quake_C" 10.0)
  (`GameplayStatics.SpawnForceFeedbackAttached` "/Game/ForceFeedback/FFE_QuakeBuildup.FFE_QuakeBuildup" _capsulecomponent "None" (0.0 0.0 0.0) (struct) "KeepRelativeOffset" false false 0.6 0.0 null)
  (`GameplayStatics.ApplyDamage` null 10.0)
  (`KismetSystemLibrary.Delay` 2.0)
  (`GameplayStatics.SpawnForceFeedbackAttached` null _capsulecomponent "None" (0.0 0.0 0.0) (struct) "KeepRelativeOffset" false false 1.5 0.0 null)
  (`LegacyCameraShake.StartLegacyCameraShake` (`GameplayStatics.GetPlayerCameraManager` 0) "/Game/CameraShake/LCS_QuakePeak.LCS_QuakePeak_C")
  (`KismetSystemLibrary.Delay` 0.2)
  (if (not (`NavMovementComponent.IsFalling` (`Character.CharacterMovement` _returnvalue)))
    (`self.Do Damage`))
  (bind _output_get (set `self.Attack Delay` (`KismetMathLibrary.RandomFloatInRange` 0.5 2.0)))
  (`KismetSystemLibrary.Delay` _output_get)
  (`self.Decide Next Attack`))

(fn `UserConstructionScript`)